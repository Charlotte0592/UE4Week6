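; Base third-person shooter character with two gun slots, interface-driven interaction, grenade launching and delayed destruction on death.
; Actor yaw follows control rotation except during Alt free look, whose release plays a timeline rotation blend before following resumes.
; Capsule overlaps notify interactables, and Interact triggers the first one found.
; PickUpGun fills empty slots or drops the equipped gun and recurses, while UpdateGunAttachments sockets equipped and stowed guns to the mesh.
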(event OnComponentBeginOverlap(CapsuleComponent)
  (params (OverlappedComponent :type Primitive%20Component%20Object%20Reference) (OtherActor :type Actor%20Object%20Reference) (OtherComp :type Primitive%20Component%20Object%20Reference) (OtherBodyIndex :type Integer) (bFromSweep :type Boolean) (SweepResult :type Hit%20Result%20Structure%20%28by%20ref%29))
  ;[1 1 1] Pick Up Gun
  (if (Utilities|DoesObjectImplementInterface OtherActor "/Game/InteractionInterface/InteractionInterface.InteractionInterface_C")
    (Class|InteractionInterface|OnInteractionRangeEntered(Message) OtherActor self)))

(event OnComponentEndOverlap(CapsuleComponent)
  (params (OverlappedComponent :type Primitive%20Component%20Object%20Reference) (OtherActor :type Actor%20Object%20Reference) (OtherComp :type Primitive%20Component%20Object%20Reference) (OtherBodyIndex :type Integer))
  ;[1 1 1] Pick Up Gun
  (if (Utilities|DoesObjectImplementInterface OtherActor "/Game/InteractionInterface/InteractionInterface.InteractionInterface_C")
    (Class|InteractionInterface|OnInteractionRangeExited(Message) OtherActor)))

(event EventTick
  (params (DeltaSeconds :type Float%20%28single-precision%29))
  ;[1 1 1] Alt自由视角切换
  (Utilities|FlowControl|Sequence
    (:then_0
      (if (not (Variables|Default|GetIsAltPressed))
        (Transformation|SetActorRotation (Math|Rotator|MakeRotator 0.0 0.0 (.yaw (Pawn|GetControlRotation :!class /Script/Engine.Pawn))))))
    (:then_1
      (if (Variables|Default|GetbIsDead)
        (Utilities|FlowControl|Delay 3.0)
        (Actor|DestroyActor)))))

(event Input|ActionEvents|InputActionInteract
  (params (Key :type Key%20Structure :default "None"))
  ;[1 1 1] Pick Up Gun
  (:Pressed
    (bind _array_element (Utilities|Array|ForEachLoopwithBreak (Collision|GetOverlappingActors (Variables|Default|GetCapsuleComponent) "/Script/Engine.Actor" :!class /Script/Engine.PrimitiveComponent) :!label _label)
      (:LoopBody
        (if (Utilities|DoesObjectImplementInterface _array_element "/Game/InteractionInterface/InteractionInterface.InteractionInterface_C")
          (Class|InteractionInterface|OnInteracted(Message) _array_element self)
          (goto _label Break))))))

(event Input|ActionEvents|InputActionSwitchGuns
  (params (Key :type Key%20Structure :default "None"))
  ;[1 1 1] Switch Guns
  (:Pressed
    (switch Utilities|FlowControl|Switch|SwitchonEGunSlot (Variables|Default|GetCurrentGunSlot)
      (:NewEnumerator0
        (Variables|Default|SetCurrentGunSlot "NewEnumerator1"))
      (:NewEnumerator1
        (Variables|Default|SetCurrentGunSlot "NewEnumerator0")))
    (Public|UpdateGunAttachments)))

(event Input|KeyboardEvents|LeftAlt
  (params (Key :type Key%20Structure :default "None"))
  (bind _springarm (Variables|Default|GetSpringArm))
  (bind _returnvalue (Class|SpringArmComponent|GetTargetRotation _springarm))
  ;[1 1 1] Alt自由视角切换
  (:Pressed
    (Variables|Default|SetIsAltPressed true)
    (Variables|Default|SetAltPressed _returnvalue))
  (:Released
    (Variables|Default|SetAltReleased _returnvalue)
    (bind _新建轨道_0 (Timeline|View PlayFromStart)
      (:Update
        (Transformation|SetActorRotation (Math|Rotator|Lerp(Rotator) (Variables|Default|GetAltReleased) (Variables|Default|GetAltPressed) _新建轨道_0 true)))
      (:Finished
        (Variables|Default|SetIsAltPressed false)))))

(event Input|KeyboardEvents|C
  (params (Key :type Key%20Structure :default "None"))
  (bind _tpscamera (Variables|Default|GetTpsCamera))
  (bind _returnvalue (Transformation|GetWorldRotation _tpscamera))
  ;[1 1 1] Grenade
  (:Pressed
    (if (not (Variables|Default|GetbIsHip))
      (bind _returnvalue_2 (Game|SpawnActorfromClass "/Game/Blueprints/Grenade.Grenade_C" (Math|Transform|MakeTransform (Transformation|GetSocketLocation (Variables|Default|GetGunWeapon) "Muzzle") _returnvalue "3.000000,3.000000,3.000000") "Undefined" 0 0))
      (Physics|SetPhysicsLinearVelocity (Variables|/Game/Blueprints/Grenade.Grenade_C|GetStaticMesh _returnvalue_2) (* (Math|Vector|GetForwardVector _returnvalue) 1e+03) false "None"))))

(fn ConstructionScript)

(fn PickUpGun
  (params (Gun :type BP%20Gun%20Object%20Reference))
  (Utilities|IsValid (Variables|Default|GetPrimaryGun)
    (:Is%20Valid
      (Utilities|IsValid (Variables|Default|GetSecondaryGun)
        (:Is%20Valid
          (bind _outputpin (Utilities|EquippedGun)
            (:Is%20Valid
              (Transformation|DetachFromActor _outputpin "KeepWorld" "KeepWorld" "KeepWorld")
              (Default|Drop _outputpin)
              (Utilities|SetEquippedGun)
              (Public|PickUpGun Gun))))
        (:Is%20Not%20Valid
          (Variables|Default|SetSecondaryGun Gun)
          (Public|UpdateGunAttachments :!label _label))))
    (:Is%20Not%20Valid
      (Variables|Default|SetPrimaryGun Gun)
      (goto _label))))

(fn UpdateGunAttachments
  (Utilities|FlowControl|Sequence
    (:then_0
      (bind _outputpin (Utilities|EquippedGun)
        (:Is%20Valid
          (Transformation|AttachComponentToComponent _outputpin (Variables|Character|GetMesh) "Weapon" "SnapToTarget" "SnapToTarget" "SnapToTarget" true))))
    (:then_1
      (bind _outputpin_2 (Utilities|StowedGun)
        (:Is%20Valid
          (Transformation|AttachComponentToComponent _outputpin_2 (Variables|Character|GetMesh) "GunStowedSocket" "SnapToTarget" "SnapToTarget" "SnapToTarget" true))))))